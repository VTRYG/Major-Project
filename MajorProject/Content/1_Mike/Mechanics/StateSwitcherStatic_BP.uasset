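; StateSwitcherStatic_BP is a placed orb that lets the player toggle their character between Normal and its configured Conflict or Avoidance state.
; The construction script picks the orb mesh from that state.
; Entering the box shows a text prompt, kept yawed toward the follow camera by a looping timer, and opens a Gate.
; While open, pressing E toggles the character's state and notifies the controller; leaving reverses this.
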(event `ShowUI`
  (bind _textrender (`self.TextRender`))
  (bind (_returnvalue_roll _returnvalue_pitch _returnvalue_yaw) (`KismetMathLibrary.BreakRotator` (`KismetMathLibrary.FindLookAtRotation` (`SceneComponent.K2_GetComponentLocation` _textrender) (`SceneComponent.K2_GetComponentLocation` (`/Game/Character/CustomCharacter.FollowCamera` (stale `self.Box.OnComponentBeginOverlap` _ascustom_character))))))
  (`SceneComponent.K2_SetRelativeRotation` _textrender (`KismetMathLibrary.MakeRotator` 0.0 0.0 _returnvalue_yaw) false false))

(event `Key|E` :consume false
  (params (Key :type "Key Structure"))
  (bind _state (`self.State`))
  (bind _controller (`self.Controller`))
  (:`Pressed`
    (`/Engine/EditorBlueprintResources/StandardMacros.Gate` true :!label _label
      (:`Exit`
        (if (`|EnumEquality` (`/Game/Character/CustomCharacter.State` (stale `self.Box.OnComponentBeginOverlap` _ascustom_character)) _state)
          (bind _output_get (set `/Game/Character/CustomCharacter.State` "NewEnumerator0" (stale `self.Box.OnComponentBeginOverlap` _ascustom_character)))
          (message `/Game/Blueprints/WorldStateInterface.ChangeState` _controller _output_get)
          (else
            (bind _output_get_2 (set `/Game/Character/CustomCharacter.State` _state (stale `self.Box.OnComponentBeginOverlap` _ascustom_character)))
            (message `/Game/Blueprints/WorldStateInterface.ChangeState` _controller _output_get_2)))))))

(event `self.Box.OnComponentBeginOverlap`
  (params (OverlappedComponent :type "PrimitiveComponent Object Reference") (OtherActor :type "Actor Object Reference") (OtherComp :type "PrimitiveComponent Object Reference") (OtherBodyIndex :type Integer) (bFromSweep :type Boolean) (SweepResult :type "HitResult Structure (by ref)"))
  (bind _ascustom_character (cast `/Game/Character/CustomCharacter` OtherActor))
  (bind _returnvalue (`KismetSystemLibrary.K2_SetTimerDelegate` (delegate `ShowUI`) 0.1 true))
  (`SceneComponent.SetVisibility` (`self.TextRender`) true false)
  (goto _label :!via `Open`))

(event `self.Box.OnComponentEndOverlap`
  (params (OverlappedComponent :type "PrimitiveComponent Object Reference") (OtherActor :type "Actor Object Reference") (OtherComp :type "PrimitiveComponent Object Reference") (OtherBodyIndex :type Integer))
  (cast `/Game/Character/CustomCharacter` OtherActor)
  (`KismetSystemLibrary.K2_ClearAndInvalidateTimerHandle` (stale `self.Box.OnComponentBeginOverlap` _returnvalue))
  (`SceneComponent.SetVisibility` (`self.TextRender`) false false)
  (goto _label :!via `Close`))

(fn `UserConstructionScript`
  (`StaticMeshComponent.SetStaticMesh` (`self.Orb`) (select `/Game/Random/State` (`self.State`) :`NewEnumerator1` "/Game/1_Mike/Models/ConflictOrb.ConflictOrb" :`NewEnumerator2` "/Game/1_Mike/Models/AvoidanceOrb.AvoidanceOrb" :!type "StaticMesh Object Reference")))