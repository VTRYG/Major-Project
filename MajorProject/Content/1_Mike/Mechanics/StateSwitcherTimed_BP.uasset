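; StateSwitcherTimed_BP is an interactable orb that temporarily switches the player character's State to its own configured State.
; Overlapping the Box shows a text prompt that turns to face the player and opens a gate for the E key.
; Pressing E sets the new state, notifies the Controller, and starts a timer that reverts the player to Normal.
; The construction script picks the orb mesh from State.
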(event `self.ReceiveTick`
  (params (DeltaSeconds :type "Float (single-precision)"))
  (bind _textrender (`self.TextRender`))
  (if (`self.Collision`)
    (bind (_returnvalue_roll _returnvalue_pitch _returnvalue_yaw) (`KismetMathLibrary.BreakRotator` (`KismetMathLibrary.FindLookAtRotation` (`SceneComponent.K2_GetComponentLocation` _textrender) (`self.K2_GetActorLocation` (stale `self.Box.OnComponentBeginOverlap` _asthird_person_character)))))
    (`SceneComponent.K2_SetRelativeRotation` _textrender (`KismetMathLibrary.MakeRotator` 0.0 0.0 _returnvalue_yaw) false false)))

(event `Key|E` :consume false
  (params (Key :type "Key Structure"))
  (bind _state (`self.State`))
  (:`Pressed`
    (`/Engine/EditorBlueprintResources/StandardMacros.Gate` true :!label _label
      (:`Exit`
        (if (not (`|EnumEquality` (`/Game/Folders/ThirdPersonBP/Blueprints/ThirdPersonCharacter.State` (stale `self.Box.OnComponentBeginOverlap` _asthird_person_character)) _state))
          (`KismetSystemLibrary.K2_SetTimerDelegate` (delegate `StartTimer`) (`self.Time`))
          (bind _output_get (set `/Game/Folders/ThirdPersonBP/Blueprints/ThirdPersonCharacter.State` _state (stale `self.Box.OnComponentBeginOverlap` _asthird_person_character)))
          (message `/Game/Blueprints/WorldStateInterface.ChangeState` (`self.Controller`) _output_get))))))

(event `self.Box.OnComponentBeginOverlap`
  (params (OverlappedComponent :type "PrimitiveComponent Object Reference") (OtherActor :type "Actor Object Reference") (OtherComp :type "PrimitiveComponent Object Reference") (OtherBodyIndex :type Integer) (bFromSweep :type Boolean) (SweepResult :type "HitResult Structure (by ref)"))
  (bind _asthird_person_character (cast `/Game/Folders/ThirdPersonBP/Blueprints/ThirdPersonCharacter` OtherActor))
  (set `self.Collision` true)
  (`SceneComponent.SetVisibility` (`self.TextRender`) true false)
  (goto _label :!via `Open`))

(event `StartTimer`
  (bind _output_get (set `/Game/Folders/ThirdPersonBP/Blueprints/ThirdPersonCharacter.State` "NewEnumerator0" (stale `self.Box.OnComponentBeginOverlap` _asthird_person_character)))
  (message `/Game/Blueprints/WorldStateInterface.ChangeState` (`self.Controller`) _output_get))

(event `self.Box.OnComponentEndOverlap`
  (params (OverlappedComponent :type "PrimitiveComponent Object Reference") (OtherActor :type "Actor Object Reference") (OtherComp :type "PrimitiveComponent Object Reference") (OtherBodyIndex :type Integer))
  (cast `/Game/Folders/ThirdPersonBP/Blueprints/ThirdPersonCharacter` OtherActor)
  (set `self.Collision` false)
  (`SceneComponent.SetVisibility` (`self.TextRender`) false false)
  (goto _label :!via `Close`))

(fn `UserConstructionScript`
  (`StaticMeshComponent.SetStaticMesh` (`self.Orb`) (select `/Game/Random/State` (`self.State`) :`NewEnumerator1` "/Game/1_Mike/ConflictOrb.ConflictOrb" :`NewEnumerator2` "/Game/1_Mike/AvoidanceOrb.AvoidanceOrb" :!type "StaticMesh Object Reference")))