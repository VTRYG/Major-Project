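; Ranged state switcher actor that gives the player character its Conflict or Avoidance state while inside an expandable pulse sphere.
; Entering the box shows text that yaws to face the character and opens a gate for E, which toggles a timeline growing or shrinking the sphere.
; Sphere overlap sets the character's state, exit restores Normal, and both message the controller.
; The construction script picks orb mesh and pulse material by state.
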(event `self.ReceiveTick`
  (params (DeltaSeconds :type "Float (single-precision)"))
  (bind _textrender (`self.TextRender`))
  (if (`self.Collision`)
    (bind (_returnvalue_roll _returnvalue_pitch _returnvalue_yaw) (`KismetMathLibrary.BreakRotator` (`KismetMathLibrary.FindLookAtRotation` (`SceneComponent.K2_GetComponentLocation` _textrender) (`self.K2_GetActorLocation` (stale `self.Box.OnComponentBeginOverlap` _ascustom_character)))))
    (`SceneComponent.K2_SetRelativeRotation` _textrender (`KismetMathLibrary.MakeRotator` 0.0 0.0 _returnvalue_yaw) false false)))

(event `Key|E` :consume false
  (params (Key :type "Key Structure"))
  (:`Pressed`
    (`/Engine/EditorBlueprintResources/StandardMacros.Gate` true :!label _label
      (:`Exit`
        (`/Engine/EditorBlueprintResources/StandardMacros.FlipFlop`
          (:`A`
            (bind (_direction _scale) (`Timeline|SphereScale` :!via `PlayFromStart` :!label _label_2)
              (:`Update`
                (`SceneComponent.SetRelativeScale3D` (`self.Sphere`) (`KismetMathLibrary.VLerp` (0.1 0.1 0.1) (* (1.0 1.0 1.0) (`self.Scale`)) _scale)))))
          (:`B`
            (goto _label_2 :!via `ReverseFromEnd`)))))))

(event `self.Box.OnComponentBeginOverlap`
  (params (OverlappedComponent :type "PrimitiveComponent Object Reference") (OtherActor :type "Actor Object Reference") (OtherComp :type "PrimitiveComponent Object Reference") (OtherBodyIndex :type Integer) (bFromSweep :type Boolean) (SweepResult :type "HitResult Structure (by ref)"))
  (bind _ascustom_character (cast `/Game/Character/CustomCharacter` OtherActor))
  (set `self.Collision` true)
  (`SceneComponent.SetVisibility` (`self.TextRender`) true false)
  (goto _label :!via `Open`))

(event `self.Box.OnComponentEndOverlap`
  (params (OverlappedComponent :type "PrimitiveComponent Object Reference") (OtherActor :type "Actor Object Reference") (OtherComp :type "PrimitiveComponent Object Reference") (OtherBodyIndex :type Integer))
  (cast `/Game/Character/CustomCharacter` OtherActor)
  (set `self.Collision` false)
  (`SceneComponent.SetVisibility` (`self.TextRender`) false false)
  (goto _label :!via `Close`))

(event `self.Sphere.OnComponentBeginOverlap`
  (params (OverlappedComponent :type "PrimitiveComponent Object Reference") (OtherActor :type "Actor Object Reference") (OtherComp :type "PrimitiveComponent Object Reference") (OtherBodyIndex :type Integer) (bFromSweep :type Boolean) (SweepResult :type "HitResult Structure (by ref)"))
  (bind _ascustom_character (cast `/Game/Character/CustomCharacter` OtherActor))
  (set `/Game/Character/CustomCharacter.State` (`self.State`) _ascustom_character)
  (message `/Game/Blueprints/WorldStateInterface.ChangeState` (`self.Controller`) "NewEnumerator0"))

(event `self.Sphere.OnComponentEndOverlap`
  (params (OverlappedComponent :type "PrimitiveComponent Object Reference") (OtherActor :type "Actor Object Reference") (OtherComp :type "PrimitiveComponent Object Reference") (OtherBodyIndex :type Integer))
  (bind _ascustom_character (cast `/Game/Character/CustomCharacter` OtherActor))
  (bind _output_get (set `/Game/Character/CustomCharacter.State` "NewEnumerator0" _ascustom_character))
  (message `/Game/Blueprints/WorldStateInterface.ChangeState` (`self.Controller`) _output_get))

(fn `UserConstructionScript`
  (bind _state (`self.State`))
  (`StaticMeshComponent.SetStaticMesh` (`self.Orb`) (select `/Game/Random/State` _state :`NewEnumerator1` "/Game/1_Mike/Models/ConflictOrb.ConflictOrb" :`NewEnumerator2` "/Game/1_Mike/Models/AvoidanceOrb.AvoidanceOrb" :!type "StaticMesh Object Reference"))
  (`PrimitiveComponent.SetMaterial` (`self.Sphere`) 0 (select `/Game/Random/State` _state :`NewEnumerator1` "/Game/1_Mike/Materials/ConflictPulse.ConflictPulse" :`NewEnumerator2` "/Game/1_Mike/Materials/AvoidancePulse.AvoidancePulse" :!type "MaterialInterface Object Reference")))