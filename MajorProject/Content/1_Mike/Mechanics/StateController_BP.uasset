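; StateController_BP switches the game between Normal, Conflict and Avoidance states and tints the screen to match.
; ChangeState relays the new state to every actor in StateActors through ChangeStateMessage, then restarts a timeline.
; The timeline lerps post-process color gain from the old state's tint to the new one: neutral, red or blue.
; OldState updates only when the timeline finishes, so an interrupted transition restarts from the last completed tint.
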(event `/Game/Blueprints/WorldStateInterface.ChangeState`
  (params (State :type "/Game/Random/State Enum" :default "NewEnumerator0"))
  (bind _newstate (`self.NewState`))
  (`|ExecutionSequence`
    (:`then_0`
      (for _array_element (`self.StateActors`)
        (message `/Game/Blueprints/WorldStateInterface.ChangeState` _array_element State)))
    (:`then_1`
      (set `self.NewState` State)
      (bind (_direction _output) (`Timeline|LerpTimeline` :!via `PlayFromStart`)
        (:`Update`
          (bind (_returnvalue_x _returnvalue_y _returnvalue_z) (`KismetMathLibrary.BreakVector` (`KismetMathLibrary.VLerp` (select `/Game/Random/State` (stale _output_get) :`NewEnumerator0` (1.0 1.0 1.0) :`NewEnumerator1` (1.5 1.0 1.0) :`NewEnumerator2` (1.0 1.0 1.5) :!type "Vector Structure") (select `/Game/Random/State` _newstate :`NewEnumerator0` (1.0 1.0 1.0) :`NewEnumerator1` (1.5 1.0 1.0) :`NewEnumerator2` (1.0 1.0 1.5) :!type "Vector Structure") _output)))
          (set `PostProcessVolume.Settings` (make `PostProcessSettings` :`ColorGain` (`KismetMathLibrary.MakeVector4` _returnvalue_x _returnvalue_y _returnvalue_z 1.0)) (`self.PostProcess`)))
        (:`Finished`
          (bind _output_get (set `self.OldState` _newstate)))))))

(fn `UserConstructionScript`)