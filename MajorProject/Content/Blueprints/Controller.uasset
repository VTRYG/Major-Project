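; Controller is an actor Blueprint that links to Input and Output actors and visualizes those connections as coloured splines.
; Its construction script adds a spline component from its own location to each linked actor, coloured by OutputColour or InputColour to show wiring in the editor.
; InputOn and InputOff loop over Output with empty bodies, so no signal is forwarded, and BeginPlay, overlap and Tick are empty.
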(event `InputOn`
  (for _ (`self.Output`)
    _))

(event `InputOff`
  (for _ (`self.Output`)
    _))

(fn `UserConstructionScript`
  (bind _input_colour (`self.Input Colour`))
  (bind _output_colour (`self.Output Colour`))
  (`|ExecutionSequence`
    (:`then_0`
      (for _array_element (`self.Output`)
        (bind _returnvalue (`AddComponent|NODE_AddSplineComponent-0`))
        (`SplineComponent.SetLocationAtSplinePoint` _returnvalue 0 (`self.K2_GetActorLocation`) "World" true)
        (`SplineComponent.SetLocationAtSplinePoint` _returnvalue 1 (`self.K2_GetActorLocation` _array_element) "World" true)
        (`SplineComponent.SetSelectedSplineSegmentColor` _returnvalue _output_colour)
        (`SplineComponent.SetUnselectedSplineSegmentColor` _returnvalue _output_colour)))
    (:`then_1`
      (for _array_element_2 (`self.Input`)
        (bind _returnvalue_2 (`AddComponent|NODE_AddSplineComponent-1`))
        (`SplineComponent.SetLocationAtSplinePoint` _returnvalue_2 0 (`self.K2_GetActorLocation`) "World" true)
        (`SplineComponent.SetLocationAtSplinePoint` _returnvalue_2 1 (`self.K2_GetActorLocation` _array_element_2) "World" true)
        (`SplineComponent.SetSelectedSplineSegmentColor` _returnvalue_2 _input_colour)
        (`SplineComponent.SetUnselectedSplineSegmentColor` _returnvalue_2 _input_colour)))))