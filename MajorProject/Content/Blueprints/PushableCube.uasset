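; PushableCube is a cube Blueprint that lets an overlapping actor push it from any of four sides.
; Each Side component's begin overlap calls BeginOverlap with the actor, the matching Arrow component and that arrow's forward vector as the push direction.
; End overlaps pass the actor to EndOverlap.
; The push logic is not in these graphs, which only route side events, and the construction script just runs the parent's.
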(event `self.Side_1.OnComponentBeginOverlap`
  (params (OverlappedComponent :type "PrimitiveComponent Object Reference") (OtherActor :type "Actor Object Reference") (OtherComp :type "PrimitiveComponent Object Reference") (OtherBodyIndex :type Integer) (bFromSweep :type Boolean) (SweepResult :type "HitResult Structure (by ref)"))
  (bind _arrow_1 (`self.Arrow_1`))
  (`self.Begin Overlap` OtherActor _arrow_1 (`SceneComponent.GetForwardVector` _arrow_1)))

(event `self.Side_1.OnComponentEndOverlap`
  (params (OverlappedComponent :type "PrimitiveComponent Object Reference") (OtherActor :type "Actor Object Reference") (OtherComp :type "PrimitiveComponent Object Reference") (OtherBodyIndex :type Integer))
  (`self.End Overlap` OtherActor))

(event `self.Side_2.OnComponentBeginOverlap`
  (params (OverlappedComponent :type "PrimitiveComponent Object Reference") (OtherActor :type "Actor Object Reference") (OtherComp :type "PrimitiveComponent Object Reference") (OtherBodyIndex :type Integer) (bFromSweep :type Boolean) (SweepResult :type "HitResult Structure (by ref)"))
  (bind _arrow_2 (`self.Arrow_2`))
  (`self.Begin Overlap` OtherActor _arrow_2 (`SceneComponent.GetForwardVector` _arrow_2)))

(event `self.Side_2.OnComponentEndOverlap`
  (params (OverlappedComponent :type "PrimitiveComponent Object Reference") (OtherActor :type "Actor Object Reference") (OtherComp :type "PrimitiveComponent Object Reference") (OtherBodyIndex :type Integer))
  (`self.End Overlap` OtherActor))

(event `self.Side_3.OnComponentBeginOverlap`
  (params (OverlappedComponent :type "PrimitiveComponent Object Reference") (OtherActor :type "Actor Object Reference") (OtherComp :type "PrimitiveComponent Object Reference") (OtherBodyIndex :type Integer) (bFromSweep :type Boolean) (SweepResult :type "HitResult Structure (by ref)"))
  (bind _arrow_3 (`self.Arrow_3`))
  (`self.Begin Overlap` OtherActor _arrow_3 (`SceneComponent.GetForwardVector` _arrow_3)))

(event `self.Side_3.OnComponentEndOverlap`
  (params (OverlappedComponent :type "PrimitiveComponent Object Reference") (OtherActor :type "Actor Object Reference") (OtherComp :type "PrimitiveComponent Object Reference") (OtherBodyIndex :type Integer))
  (`self.End Overlap` OtherActor))

(event `self.Side_4.OnComponentBeginOverlap`
  (params (OverlappedComponent :type "PrimitiveComponent Object Reference") (OtherActor :type "Actor Object Reference") (OtherComp :type "PrimitiveComponent Object Reference") (OtherBodyIndex :type Integer) (bFromSweep :type Boolean) (SweepResult :type "HitResult Structure (by ref)"))
  (bind _arrow_4 (`self.Arrow_4`))
  (`self.Begin Overlap` OtherActor _arrow_4 (`SceneComponent.GetForwardVector` _arrow_4)))

(event `self.Side_4.OnComponentEndOverlap`
  (params (OverlappedComponent :type "PrimitiveComponent Object Reference") (OtherActor :type "Actor Object Reference") (OtherComp :type "PrimitiveComponent Object Reference") (OtherBodyIndex :type Integer))
  (`self.End Overlap` OtherActor))

(fn `UserConstructionScript`
  (`parent.UserConstructionScript`))