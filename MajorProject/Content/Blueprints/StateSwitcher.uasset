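; StateSwitcher is an interactable actor that toggles the third-person character's State while the character stands inside its Box.
; Box overlap begin and end open and close a gate on the E key, and the begin event caches the overlapping character.
; Pressing E sets the character to this actor's State, or back to the enum's NewEnumerator0 if already in it.
; An unconnected loop calling ChangeToConflictStateMessage never runs.
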(event `Key|E` :consume false
  (params (Key :type "Key Structure"))
  (bind _state (`self.State`))
  (:`Pressed`
    (`/Engine/EditorBlueprintResources/StandardMacros.Gate` true :!label _label
      (:`Exit`
        (if (`|EnumEquality` (`/Game/Folders/ThirdPersonBP/Blueprints/ThirdPersonCharacter.State` (stale `self.Box.OnComponentBeginOverlap` _asthird_person_character)) _state)
          (set `/Game/Folders/ThirdPersonBP/Blueprints/ThirdPersonCharacter.State` "NewEnumerator0" (stale `self.Box.OnComponentBeginOverlap` _asthird_person_character))
          (else
            (set `/Game/Folders/ThirdPersonBP/Blueprints/ThirdPersonCharacter.State` _state (stale `self.Box.OnComponentBeginOverlap` _asthird_person_character))))))))

(event `self.Box.OnComponentBeginOverlap`
  (params (OverlappedComponent :type "PrimitiveComponent Object Reference") (OtherActor :type "Actor Object Reference") (OtherComp :type "PrimitiveComponent Object Reference") (OtherBodyIndex :type Integer) (bFromSweep :type Boolean) (SweepResult :type "HitResult Structure (by ref)"))
  (bind _asthird_person_character (cast `/Game/Folders/ThirdPersonBP/Blueprints/ThirdPersonCharacter` OtherActor))
  (goto _label :!via `Open`))

(event `self.Box.OnComponentEndOverlap`
  (params (OverlappedComponent :type "PrimitiveComponent Object Reference") (OtherActor :type "Actor Object Reference") (OtherComp :type "PrimitiveComponent Object Reference") (OtherBodyIndex :type Integer))
  (cast `/Game/Folders/ThirdPersonBP/Blueprints/ThirdPersonCharacter` OtherActor)
  (goto _label :!via `Close`))

(fn `UserConstructionScript`)