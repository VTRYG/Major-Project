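; Platform actor that is solid and visible only while the player's ThirdPersonCharacter is in the same State as the platform (Normal, Conflict or Avoidance).
; BeginPlay tints the mesh by the platform's State and starts a looping timer that polls the character through ChangeStates.
; Each poll toggles mesh collision and the Opacity material parameter on a state match.
; ChangetoConflictState is an empty stub.
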(event `self.ReceiveBeginPlay`
  (`KismetSystemLibrary.K2_SetTimerDelegate` (delegate `Change States`) 0.1 true)
  (`MeshComponent.SetVectorParameterValueOnMaterials` (`self.StaticMesh`) "Colour" (select `/Game/Random/State` (`self.State`) :`NewEnumerator1` (0.11 0.0 0.0) :`NewEnumerator2` (0.0 0.0 0.11) :!type "Vector Structure")))

(event `/Game/Blueprints/WorldStateInterface.ChangeToConflictState`
  (params (NewParam :type Boolean)))

(event `Change States`
  (bind _asthird_person_character (cast `/Game/Folders/ThirdPersonBP/Blueprints/ThirdPersonCharacter` (`GameplayStatics.GetPlayerCharacter` 0)))
  (bind _returnvalue (`|EnumEquality` (`/Game/Folders/ThirdPersonBP/Blueprints/ThirdPersonCharacter.State` _asthird_person_character) (`self.State`)))
  (`PrimitiveComponent.SetCollisionEnabled` (`self.StaticMesh`) (select `bool` _returnvalue :`false` "NoCollision" :`true` "QueryAndPhysics" :!type "ECollisionEnabled Enum"))
  (`MeshComponent.SetScalarParameterValueOnMaterials` (`self.StaticMesh`) "Opacity" (select `bool` _returnvalue :`true` 1.0 :!type "Float (single-precision)")))

(fn `UserConstructionScript`)