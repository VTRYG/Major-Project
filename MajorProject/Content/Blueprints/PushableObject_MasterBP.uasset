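; Master Blueprint for pushable objects that tracks when the player's custom character is in range to push.
; Its BeginOverlap event stores the supplied hands and interactable references, then, if the character is not already pushing, sets a collision flag, stores the object reference and passes the push direction to the character.
; EndOverlap clears the flag when that character leaves.
; The push movement itself is not implemented here.
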(event `Begin Overlap`
  (params (`Other Actor` :type "Actor Object Reference") (`Object Reference` :type "SceneComponent Object Reference") (`Push Direction` :type "Vector Structure") (Interactable :type Boolean) (`Hands Reference` :type "SceneComponent Object Reference"))
  (bind _ascustom_character (cast `/Game/Character/CustomCharacter` `Other Actor`))
  (set `self.Hands` `Hands Reference`)
  (set `self.Interactable` Interactable)
  (if (not (`/Game/Character/CustomCharacter.IsPushingObject` _ascustom_character))
    (set `self.Collision` true)
    (set `self.ObjectReference` `Object Reference`)
    (set `/Game/Character/CustomCharacter.PushDirection` `Push Direction` _ascustom_character)))

(event `End Overlap`
  (params (`Other Actor` :type "Actor Object Reference"))
  (cast `/Game/Character/CustomCharacter` `Other Actor`)
  (set `self.Collision` false))

(fn `UserConstructionScript`)