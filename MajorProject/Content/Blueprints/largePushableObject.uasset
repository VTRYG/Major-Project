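; A large pushable object with a handle on each of two sides, tinted by its Normal, Conflict or Avoidance state.
; Normal objects are always interactable; otherwise a state comparison, re-run on ChangeState, sets interactability and handle opacity.
; Each side's overlap passes its arrow, push direction and hands reference to BeginOverlap.
; A looping timer shows that side's text when interactable and yaws it toward the character's camera until overlap ends.
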(event `UI`
  (bind _returnvalue (select `int` (`self.UI_index`) :`0` (`self.Text_Side1`) :`1` (`self.Text_Side2`)))
  (if (`self.InteractableHandle`)
    (`SceneComponent.SetVisibility` _returnvalue true false)
    (bind (_returnvalue_roll _returnvalue_pitch _returnvalue_yaw) (`KismetMathLibrary.BreakRotator` (`KismetMathLibrary.FindLookAtRotation` (`SceneComponent.K2_GetComponentLocation` _returnvalue) (`SceneComponent.K2_GetComponentLocation` (`/Game/Character/CustomCharacter.FollowCamera` (stale `self.Side_1.OnComponentBeginOverlap` _ascustom_character))))))
    (`SceneComponent.K2_SetRelativeRotation` _returnvalue (`KismetMathLibrary.MakeRotator` 0.0 0.0 (- _returnvalue_yaw -90.0)) false false)))

(event `self.ReceiveBeginPlay`
  (bind _state (`self.State`))
  (if (`|EnumEquality` _state "NewEnumerator0") :!label _label
    (set `self.InteractableHandle` true)
    (else
      (bind _returnvalue (`|EnumEquality` (stale `/Game/Blueprints/WorldStateInterface.ChangeState` State) _state))
      (set `self.InteractableHandle` _returnvalue)
      (`MeshComponent.SetScalarParameterValueOnMaterials` (`self.Handle-Side1`) "Opacity" (select `bool` _returnvalue :`false` 0.2 :`true` 1.0 :!type "Float (single-precision)"))
      (`MeshComponent.SetScalarParameterValueOnMaterials` (`self.Handle-Side2`) "Opacity" (select `bool` _returnvalue :`false` 0.2 :`true` 1.0 :!type "Float (single-precision)")))))

(event `/Game/Blueprints/WorldStateInterface.ChangeState`
  (params (State :type "/Game/Random/State Enum" :default "NewEnumerator0"))
  (goto _label))

(event `self.Side_1.OnComponentBeginOverlap`
  (params (OverlappedComponent :type "PrimitiveComponent Object Reference") (OtherActor :type "Actor Object Reference") (OtherComp :type "PrimitiveComponent Object Reference") (OtherBodyIndex :type Integer) (bFromSweep :type Boolean) (SweepResult :type "HitResult Structure (by ref)"))
  (bind _arrow_1 (`self.Arrow_1`))
  (set `self.UI_index` 0)
  (`self.Begin Overlap` OtherActor _arrow_1 (`SceneComponent.GetForwardVector` _arrow_1) (`self.InteractableHandle`) (`self.Hands-Side1`))
  (bind _ascustom_character (cast `/Game/Character/CustomCharacter` (select `int` (`self.UI_index`) :`0` OtherActor :`1` (stale `self.Side_2.OnComponentBeginOverlap` OtherActor)) :!label _label_2))
  (bind _returnvalue (`KismetSystemLibrary.K2_SetTimerDelegate` (delegate `UI`) 0.1 true)))

(event `self.Side_1.OnComponentEndOverlap`
  (params (OverlappedComponent :type "PrimitiveComponent Object Reference") (OtherActor :type "Actor Object Reference") (OtherComp :type "PrimitiveComponent Object Reference") (OtherBodyIndex :type Integer))
  (`self.End Overlap` OtherActor)
  (`KismetSystemLibrary.K2_ClearAndInvalidateTimerHandle` (stale `self.Side_1.OnComponentBeginOverlap` _returnvalue) :!label _label_3)
  (`SceneComponent.SetVisibility` (select `int` (`self.UI_index`) :`0` (`self.Text_Side1`) :`1` (`self.Text_Side2`)) false false))

(event `self.Side_2.OnComponentEndOverlap`
  (params (OverlappedComponent :type "PrimitiveComponent Object Reference") (OtherActor :type "Actor Object Reference") (OtherComp :type "PrimitiveComponent Object Reference") (OtherBodyIndex :type Integer))
  (`self.End Overlap` OtherActor)
  (goto _label_3))

(event `self.Side_2.OnComponentBeginOverlap`
  (params (OverlappedComponent :type "PrimitiveComponent Object Reference") (OtherActor :type "Actor Object Reference") (OtherComp :type "PrimitiveComponent Object Reference") (OtherBodyIndex :type Integer) (bFromSweep :type Boolean) (SweepResult :type "HitResult Structure (by ref)"))
  (bind _arrow_2 (`self.Arrow_2`))
  (set `self.UI_index` 1)
  (`self.Begin Overlap` OtherActor _arrow_2 (`SceneComponent.GetForwardVector` _arrow_2) (`self.InteractableHandle`) (`self.Hands-Side2`))
  (goto _label_2))

(fn `UserConstructionScript`
  (`MeshComponent.SetVectorParameterValueOnMaterials` (`self.Handle-Side1`) "Colour" (select `/Game/Random/State` (`self.State`) :`NewEnumerator0` (1.0 1.0 1.0) :`NewEnumerator1` (0.11 0.0 0.0) :`NewEnumerator2` (0.0 0.0 0.11) :!type "Vector Structure"))
  (`MeshComponent.SetVectorParameterValueOnMaterials` (`self.Handle-Side2`) "Colour" (select `/Game/Random/State` (`self.State`) :`NewEnumerator0` (1.0 1.0 1.0) :`NewEnumerator1` (0.11 0.0 0.0) :`NewEnumerator2` (0.0 0.0 0.11) :!type "Vector Structure"))
  (`parent.UserConstructionScript`))